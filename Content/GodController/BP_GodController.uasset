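; God-view player controller actor that orbits and zooms a boom camera and casts Rockslide, Tornado and Thunderstorm abilities at the mouse cursor.
; Tick clamps pitch and moves the cursor marker to the trace hit, hiding it during rotation.
; Tornado takes two clicks, setting location then direction with an arrow.
; Cast functions spawn ability actors against limited counts, though Thunderstorm decrements the tornado count and all three clear RockslidesEnabled.
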(event Custom|Set%20Current%20Ability
  (params (Ability :type Enum_Abilities%20Enum :default "NewEnumerator0"))
  ;[1 1 1] Set Current Ability
  (bind _output_get (Variables|Default|SetCurrentAbility Ability))
  (Development|PrintString (Utilities|String|Append "Ability Chosen: " (Utilities|String|EnumtoString _output_get)) true true "(R=0.000000,G=1.000000,B=0.176122,A=1.000000)" 3.0))

(event EventBeginPlay
  ;[1 1 1] BeginPlay
  (Variables|/Script/Engine.PlayerController|SetbShowMouseCursor (Game|GetPlayerController 0) true)
  (Input|SetInputModeGameandUI (Game|GetPlayerController 0) 0 "LockOnCapture" true))

(event EventTick
  (params (DeltaSeconds :type Float%20%28single-precision%29))
  (bind _returnvalue (Game|GetPlayerController 0))
  (bind _returnvalue_2 (Game|GetPlayerController 0))
  (bind _arrow (Variables|Default|GetArrow))
  (bind _hitresult (Game|Player|GetHitResultUnderCursorbyChannel _returnvalue "TraceTypeQuery1" true))
  (bind _hitresult_2 (Game|Player|GetHitResultUnderCursorbyChannel _returnvalue_2 "TraceTypeQuery1" true))
  (bind _returnvalue_3 (Transformation|GetWorldLocation _arrow))
  (bind _location (Collision|BreakHitResult _hitresult))
  (bind _location_2 (Collision|BreakHitResult _hitresult_2))
  (bind _returnvalue_4 (- _location_2 _returnvalue_3))
  (Utilities|FlowControl|Sequence
    (:then_0
      ;[1 1 1] Tick
      (CallFunction|CameraRotationClamp)
      (if (Variables|Default|GetCameraRotationUnlocked)
        (Development|SetHiddeninGame (Variables|Default|GetCursor) true true)
        (else
          (Collision|MultiLineTraceByChannel _location (+ _location "0,0,800.000000") "TraceTypeQuery1" false 0 "None")
          (Transformation|SetWorldLocationAndRotation (Variables|Default|GetCursor) _location "0, 0, 0" false false)
          (Development|SetHiddeninGame (Variables|Default|GetCursor) false true))))
    (:then_1
      (if (Variables|Default|GetDirectionalAbilityInitiate)
        (Transformation|SetWorldLocationAndRotation (Variables|Default|GetArrow) (Variables|Default|GetCastLocation) (Math|Rotator|MakeRotfromX _returnvalue_4) false false)
        (Variables|Default|SetCastDirection (Math|Vector|Normalize (Math|Vector|ProjectVectorontoPlane _returnvalue_4 "0, 0,1.000000")))))))

(event Input|ActionEvents|InputActionRotateCam
  (params (Key :type Key%20Structure :default "None"))
  (bind _returnvalue (Game|GetPlayerController 0))
  (bind (_sizex _sizey) (HUD|GetViewportSize _returnvalue))
  ;[1 1 1] Camera Rotation
  (:Pressed
    (Variables|Default|SetCameraRotationUnlocked true))
  (:Released
    (Variables|Default|SetCameraRotationUnlocked false)
    (Class|PlayerController|SetMouseLocation _returnvalue (/ _sizex 2) (/ _sizey 2))))

(event Input|ActionEvents|InputActionZoomIn
  (params (Key :type Key%20Structure :default "None"))
  ;[1 1 1] Camera Zoom
  (:Pressed
    (CallFunction|Zoom -2e+02)))

(event Input|ActionEvents|InputActionZoomOut
  (params (Key :type Key%20Structure :default "None"))
  ;[1 1 1] Camera Zoom
  (:Pressed
    (CallFunction|Zoom 2e+02)))

(event Input|ActionEvents|InputActionPlaceAbility
  (params (Key :type Key%20Structure :default "None"))
  (bind _arrow (Variables|Default|GetArrow))
  (bind _cursor (Variables|Default|GetCursor))
  (:Pressed
    (if (Variables|Default|GetDirectionalAbilityInitiate)
      _
      (else
        (Variables|Default|SetCastLocation (.Location (Collision|BreakHitResult (.HitResult (Game|Player|GetHitResultUnderCursorbyChannel (Game|GetPlayerController 0) "TraceTypeQuery1" true)))))))
    (switch Utilities|FlowControl|Switch|SwitchonEnum_Abilities (Variables|Default|GetCurrentAbility)
      (:NewEnumerator0
        (CallFunction|CastRockslide (Variables|Default|GetCastLocation) "0, 0, 0" 25))
      (:NewEnumerator1
        (if (Variables|Default|GetDirectionalAbilityInitiate)
          (CallFunction|CastTornado (Variables|Default|GetCastLocation) "0, 0, 0" 10 (Variables|Default|GetCastDirection))
          (Variables|Default|SetDirectionalAbilityInitiate false)
          (Rendering|SetVisibility _arrow false false)
          (Rendering|SetVisibility _cursor true true)
          (else
            (Variables|Default|SetDirectionalAbilityInitiate true)
            (Rendering|SetVisibility _arrow true false)
            (Rendering|SetVisibility _cursor false true))))
      (:NewEnumerator2
        (CallFunction|CastThunderstorm (Variables|Default|GetCastLocation) "0, 0, 0" 5)))))

(event Input|MouseEvents|MouseX
  (params (AxisValue :type Float%20%28single-precision%29))
  ;[1 1 1] Camera Rotation
  (if (Variables|Default|GetCameraRotationUnlocked)
    (Class|Actor|AddActorWorldRotation (Math|Rotator|MakeRotator 0.0 0.0 (* AxisValue (Variables|Default|GetRotation%20Speed))))))

(event Input|MouseEvents|MouseY
  (params (AxisValue :type Float%20%28single-precision%29))
  ;[1 1 1] Camera Rotation
  (if (Variables|Default|GetCameraRotationUnlocked)
    (Transformation|AddActorLocalRotation (Math|Rotator|MakeRotator 0.0 (* AxisValue (Variables|Default|GetRotation%20Speed)) 0.0) false false)))

(fn ConstructionScript)

(fn CameraRotationClamp
  (bind _returnvalue (Transformation|GetActorRotation))
  (bind _returnvalue_2 (< (.pitch _returnvalue) -8e+01))
  (if (or _returnvalue_2 (> (.pitch _returnvalue) -1e+01))
    (Transformation|SetActorRotation (Math|Rotator|MakeRotator 0.0 (Math|Float|SelectFloat -8e+01 -1e+01 _returnvalue_2) (.yaw _returnvalue)))))

(fn Zoom
  (params (Zoom%20Speed :type Float%20%28double-precision%29))
  (if (not (or (> (+ (Variables|/Script/Engine.SpringArmComponent|GetTargetArmLength (Variables|Default|GetCameraBoom)) Zoom%20Speed) (Variables|Default|GetMax%20Arm%20Length)) (< (+ (Variables|/Script/Engine.SpringArmComponent|GetTargetArmLength (Variables|Default|GetCameraBoom)) Zoom%20Speed) (Variables|Default|GetMin%20Arm%20Length))))
    (Variables|/Script/Engine.SpringArmComponent|SetTargetArmLength (Variables|Default|GetCameraBoom) (+ (Variables|/Script/Engine.SpringArmComponent|GetTargetArmLength (Variables|Default|GetCameraBoom)) Zoom%20Speed))))

(fn CastRockslide
  (params (Hit%20Location :type Vector) (Hit%20Normal :type Vector) (NumberOfRocks :type Integer))
  (if (not (<= (Variables|Default|GetNumOfRockslides) 0))
    (bind _returnvalue (Game|SpawnActorfromClass "/Game/Abilities/Rockslide/BP_Ability_Rockslide.BP_Ability_Rockslide_C" (Math|Transform|MakeTransform Hit%20Location) "Undefined" 0 0))
    (Variables|/Game/Abilities/Rockslide/BP_Ability_Rockslide.BP_Ability_Rockslide_C|SetNumberOfRocks _returnvalue NumberOfRocks)
    (Variables|/Game/Abilities/Rockslide/BP_Ability_Rockslide.BP_Ability_Rockslide_C|SetLocation _returnvalue Hit%20Location)
    (Math|Integer|DecrementInt (Variables|Default|GetNumOfRockslides)
      (:%20%20
        (if (<= (Variables|Default|GetNumOfRockslides) 0)
          (Variables|Default|SetRockslidesEnabled false))))))

(fn CastTornado
  (params (Hit%20Location :type Vector) (Hit%20Normal :type Vector) (TornadoDamageValue :type Integer) (InitialDirection :type Vector))
  (if (not (<= (Variables|Default|GetNumOfTornadoes) 0))
    (bind _returnvalue (Game|SpawnActorfromClass "/Game/Abilities/Tornado/BP_Ability_Tornado.BP_Ability_Tornado_C" (Math|Transform|MakeTransform Hit%20Location) "Undefined" 0 0))
    (Variables|/Game/Abilities/Tornado/BP_Ability_Tornado.BP_Ability_Tornado_C|SetDamageValue _returnvalue TornadoDamageValue)
    (Variables|/Game/Abilities/Tornado/BP_Ability_Tornado.BP_Ability_Tornado_C|SetLocation _returnvalue Hit%20Location)
    (Variables|/Game/Abilities/Tornado/BP_Ability_Tornado.BP_Ability_Tornado_C|SetInitialDirection _returnvalue InitialDirection)
    (Math|Integer|DecrementInt (Variables|Default|GetNumOfTornadoes)
      (:%20%20
        (if (<= (Variables|Default|GetNumOfTornadoes) 0)
          (Variables|Default|SetRockslidesEnabled false))))))

(fn CastThunderstorm
  (params (Hit%20Location :type Vector) (Hit%20Normal :type Vector) (NumberOfStrikes :type Integer))
  (if (not (<= (Variables|Default|GetNumOfThunderstorms) 0))
    (bind _returnvalue (Game|SpawnActorfromClass "/Game/Abilities/Thunderstorm/BP_Ability_Thunderstorm.BP_Ability_Thunderstorm_C" (Math|Transform|MakeTransform Hit%20Location) "Undefined" 0 0))
    (Variables|/Game/Abilities/Thunderstorm/BP_Ability_Thunderstorm.BP_Ability_Thunderstorm_C|SetNumberOfStrikes _returnvalue NumberOfStrikes)
    (Variables|/Game/Abilities/Thunderstorm/BP_Ability_Thunderstorm.BP_Ability_Thunderstorm_C|SetLocation _returnvalue Hit%20Location)
    (Math|Integer|DecrementInt (Variables|Default|GetNumOfTornadoes)
      (:%20%20
        (if (<= (Variables|Default|GetNumOfTornadoes) 0)
          (Variables|Default|SetRockslidesEnabled false))))))