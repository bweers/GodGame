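; Main menu version of the god controller pawn that slowly orbits the camera behind the menu.
; BeginPlay shows the cursor, sets UI-only input and starts a looping timer that yaws the actor by RotationSpeed.
; Gameplay logic for camera control, cursor targeting and Rockslide, Tornado and Thunderstorm casting remains but is disconnected, with input events and Tick left empty.
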(event Custom|Set%20Current%20Ability
  (params (Ability :type Enum_Abilities%20Enum :default "NewEnumerator0"))
  ;[1 1 1] Set Current Ability
)

(event Custom|RotateCamera
  (Class|Actor|AddActorWorldRotation (Math|Rotator|MakeRotator 0.0 0.0 (Variables|Default|GetRotation%20Speed))))

(event EventBeginPlay
  ;[1 1 1] BeginPlay
  (Variables|/Script/Engine.PlayerController|SetbShowMouseCursor (Game|GetPlayerController 0) true)
  (Input|SetInputModeUIOnly (Game|GetPlayerController 0) 0 "DoNotLock")
  (Utilities|Time|SetTimerbyEvent (delegate Custom|RotateCamera) 0.01 true))

(event EventTick
  (params (DeltaSeconds :type Float%20%28single-precision%29)))

(event Input|ActionEvents|InputActionRotateCam
  (params (Key :type Key%20Structure :default "None"))
  ;[1 1 1] Camera Rotation
)

(event Input|ActionEvents|InputActionZoomIn
  (params (Key :type Key%20Structure :default "None"))
  ;[1 1 1] Camera Zoom
)

(event Input|ActionEvents|InputActionZoomOut
  (params (Key :type Key%20Structure :default "None"))
  ;[1 1 1] Camera Zoom
)

(event Input|ActionEvents|InputActionPlaceAbility
  (params (Key :type Key%20Structure :default "None")))

(event Input|MouseEvents|MouseX
  (params (AxisValue :type Float%20%28single-precision%29))
  ;[1 1 1] Camera Rotation
)

(event Input|MouseEvents|MouseY
  (params (AxisValue :type Float%20%28single-precision%29))
  ;[1 1 1] Camera Rotation
)

(fn ConstructionScript)

(fn CameraRotationClamp
  (bind _returnvalue (Transformation|GetActorRotation))
  (bind _returnvalue_2 (< (.pitch _returnvalue) -8e+01))
  (if (or _returnvalue_2 (> (.pitch _returnvalue) -1e+01))
    (Transformation|SetActorRotation (Math|Rotator|MakeRotator 0.0 (Math|Float|SelectFloat -8e+01 -1e+01 _returnvalue_2) (.yaw _returnvalue)))))

(fn Zoom
  (params (Zoom%20Speed :type Float%20%28double-precision%29))
  (if (not (or (> (+ (Variables|/Script/Engine.SpringArmComponent|GetTargetArmLength (Variables|Default|GetCameraBoom)) Zoom%20Speed) (Variables|Default|GetMax%20Arm%20Length)) (< (+ (Variables|/Script/Engine.SpringArmComponent|GetTargetArmLength (Variables|Default|GetCameraBoom)) Zoom%20Speed) (Variables|Default|GetMin%20Arm%20Length))))
    (Variables|/Script/Engine.SpringArmComponent|SetTargetArmLength (Variables|Default|GetCameraBoom) (+ (Variables|/Script/Engine.SpringArmComponent|GetTargetArmLength (Variables|Default|GetCameraBoom)) Zoom%20Speed))))

(fn CastRockslide
  (params (Hit%20Location :type Vector) (Hit%20Normal :type Vector) (NumberOfRocks :type Integer))
  (if (not (<= (Variables|Default|GetNumOfRockslides) 0))
    (bind _returnvalue (Game|SpawnActorfromClass "/Game/Abilities/Rockslide/BP_Ability_Rockslide.BP_Ability_Rockslide_C" (Math|Transform|MakeTransform Hit%20Location) "Undefined" 0 0))
    (Variables|/Game/Abilities/Rockslide/BP_Ability_Rockslide.BP_Ability_Rockslide_C|SetNumberOfRocks _returnvalue NumberOfRocks)
    (Variables|/Game/Abilities/Rockslide/BP_Ability_Rockslide.BP_Ability_Rockslide_C|SetLocation _returnvalue Hit%20Location)
    (Math|Integer|DecrementInt (Variables|Default|GetNumOfRockslides)
      (:%20%20
        (if (<= (Variables|Default|GetNumOfRockslides) 0)
          (Variables|Default|SetRockslidesEnabled false))))))

(fn CastTornado
  (params (Hit%20Location :type Vector) (Hit%20Normal :type Vector) (TornadoDamageValue :type Integer) (InitialDirection :type Vector))
  (if (not (<= (Variables|Default|GetNumOfTornadoes) 0))
    (bind _returnvalue (Game|SpawnActorfromClass "/Game/Abilities/Tornado/BP_Ability_Tornado.BP_Ability_Tornado_C" (Math|Transform|MakeTransform Hit%20Location) "Undefined" 0 0))
    (Variables|/Game/Abilities/Tornado/BP_Ability_Tornado.BP_Ability_Tornado_C|SetDamageValue _returnvalue TornadoDamageValue)
    (Variables|/Game/Abilities/Tornado/BP_Ability_Tornado.BP_Ability_Tornado_C|SetLocation _returnvalue Hit%20Location)
    (Variables|/Game/Abilities/Tornado/BP_Ability_Tornado.BP_Ability_Tornado_C|SetInitialDirection _returnvalue InitialDirection)
    (Math|Integer|DecrementInt (Variables|Default|GetNumOfTornadoes)
      (:%20%20
        (if (<= (Variables|Default|GetNumOfTornadoes) 0)
          (Variables|Default|SetRockslidesEnabled false))))))

(fn CastThunderstorm
  (params (Hit%20Location :type Vector) (Hit%20Normal :type Vector) (NumberOfStrikes :type Integer))
  (if (not (<= (Variables|Default|GetNumOfThunderstorms) 0))
    (bind _returnvalue (Game|SpawnActorfromClass "/Game/Abilities/Thunderstorm/BP_Ability_Thunderstorm.BP_Ability_Thunderstorm_C" (Math|Transform|MakeTransform Hit%20Location) "Undefined" 0 0))
    (Variables|/Game/Abilities/Thunderstorm/BP_Ability_Thunderstorm.BP_Ability_Thunderstorm_C|SetNumberOfStrikes _returnvalue NumberOfStrikes)
    (Variables|/Game/Abilities/Thunderstorm/BP_Ability_Thunderstorm.BP_Ability_Thunderstorm_C|SetLocation _returnvalue Hit%20Location)
    (Math|Integer|DecrementInt (Variables|Default|GetNumOfTornadoes)
      (:%20%20
        (if (<= (Variables|Default|GetNumOfTornadoes) 0)
          (Variables|Default|SetRockslidesEnabled false))))))