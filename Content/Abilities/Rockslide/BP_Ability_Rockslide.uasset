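; Rockslide ability actor that scatters a batch of randomly rotated and scaled BP_Rock actors around its location, then destroys itself.
; One tick after BeginPlay, it raises SpawnArea above itself and runs a ForLoopWithDelay over NumberOfRocks.
; Each iteration traces downward from random points in a box overhead and spawns a rock slightly off the hit surface along its normal.
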(event EventBeginPlay
  (bind _returnvalue (Math|Random|RandomFloatinRange 0.15 0.25))
  (bind _location (Variables|Default|GetLocation))
  (bind _returnvalue_2 (+ _location "0,0,1000.000000"))
  (bind _returnvalue_3 (Math|Random|RandomPointinBoundingBox _returnvalue_2 "250.000000,250.000000,1.000000"))
  (Utilities|FlowControl|DelayUntilNextTick)
  (Transformation|SetWorldLocation (Variables|Default|GetSpawnArea) (+ (Variables|Default|GetLocation) "0,0,1000.000000") false false)
  (Utilities|ForLoopwithDelay 0 (- (Variables|Default|GetNumberOfRocks) 1) 0.0
    (:Loop%20Body
      (bind _outhit (Collision|LineTraceByChannel _returnvalue_3 (- _returnvalue_3 "0,0,1500.000000") "TraceTypeQuery1" false 0 "None"))
      (Game|SpawnActorfromClass "/Game/Abilities/Rockslide/BP_Rock.BP_Rock_C" (Math|Transform|MakeTransform (+ (.Location (Collision|BreakHitResult _outhit)) (* (.Normal (Collision|BreakHitResult _outhit)) 75.0)) (Math|Random|RandomRotator false) (Math|Vector|MakeVector _returnvalue _returnvalue _returnvalue)) "Undefined" 0 0))
    (:Completed
      (Actor|DestroyActor))))

(fn ConstructionScript)