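; Rock actor for the Rockslide ability that damages destructible structures and removes itself once it comes to rest.
; Static mesh hits on destructible structures pass the rock's current speed to their velocity-based damage function.
; A looping timer started on BeginPlay periodically checks speed and destroys the rock when it is nearly stationary.
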(event OnComponentHit(StaticMesh)
  (params (HitComponent :type Primitive%20Component%20Object%20Reference) (OtherActor :type Actor%20Object%20Reference) (OtherComp :type Primitive%20Component%20Object%20Reference) (NormalImpulse :type Vector :default "0, 0, 0") (Hit :type Hit%20Result%20Structure%20%28by%20ref%29))
  (bind _asbp_structure_destructible (Utilities|Casting|CastToBP_Structure_Destructible OtherActor))
  (Default|ApplyDamageVelocity _asbp_structure_destructible (Math|Vector|VectorLength (Transformation|GetVelocity))))

(event Custom|DestroyTimer
  (if (< (Math|Vector|VectorLength (Transformation|GetVelocity)) 15.0)
    (Actor|DestroyActor)))

(event EventBeginPlay
  (Utilities|Time|SetTimerbyEvent (delegate Custom|DestroyTimer) 5.0 true))

(fn ConstructionScript)