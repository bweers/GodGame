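; Thunderstorm ability actor that strikes an area with a series of lightning bolts, then destroys itself.
; On BeginPlay it waits a tick, raises SpawnArea above Location, and runs a randomly delayed loop for NumberOfStrikes.
; Each iteration traces downward between independently random points, producing slanted lines.
; It spawns BP_LightningStrike offset along the hit normal and a randomly yawed burn decal at the hit point.
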(event EventBeginPlay
  (bind _spawnarea (Variables|Default|GetSpawnArea))
  (bind _returnvalue (Transformation|GetWorldLocation _spawnarea))
  (bind _returnvalue_2 (Math|Random|RandomPointinBoundingBox _returnvalue "300.000000,300.000000,1.000000"))
  (Utilities|FlowControl|DelayUntilNextTick)
  (Transformation|SetWorldLocation _spawnarea (+ (Variables|Default|GetLocation) "0,0,1000.000000") false false)
  (Utilities|ForLoopwithDelay 0 (- (Variables|Default|GetNumberOfStrikes) 1) (Math|Random|RandomFloatinRange 0.5 3.0)
    (:Loop%20Body
      (bind _outhit (Collision|LineTraceByChannel _returnvalue_2 (- _returnvalue_2 "0,0,1500.000000") "TraceTypeQuery1" false 0 "None"))
      (Game|SpawnActorfromClass "/Game/Abilities/Thunderstorm/BP_LightningStrike.BP_LightningStrike_C" (Math|Transform|MakeTransform (+ (.Location (Collision|BreakHitResult _outhit)) (* (.Normal (Collision|BreakHitResult _outhit)) 75.0)) "0, 0, 0" (Math|Vector|MakeVector 1.0 1.0 1.0)) "Undefined" 0 0)
      (Rendering|Decal|SpawnDecalatLocation "/Game/EnvironmentActors/Decals/MAT_BurnMark.MAT_BurnMark" "180.000000,180.000000,180.000000" (.Location (Collision|BreakHitResult _outhit)) (Math|Rotator|MakeRotator 0.0 -9e+01 (Math|Random|RandomFloatinRange -1.5e+02 1.5e+02)) 0.0))
    (:Completed
      (Actor|DestroyActor))))

(fn ConstructionScript)