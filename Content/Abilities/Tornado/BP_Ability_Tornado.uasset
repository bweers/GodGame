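; Tornado ability actor that wanders across the terrain and damages destructible structures until its lifetime expires.
; A looping timer steps it along CurrentDirection, snapping to ground via downward traces and picking a random new InitialDirection on a miss.
; Tick occasionally applies Perlin-noise yaw around InitialDirection to vary the path.
; Capsule overlaps start and stop tornado damage on structures; the start call is marked not working.
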(event OnComponentBeginOverlap(Capsule)
  (params (OverlappedComponent :type Primitive%20Component%20Object%20Reference) (OtherActor :type Actor%20Object%20Reference) (OtherComp :type Primitive%20Component%20Object%20Reference) (OtherBodyIndex :type Integer) (bFromSweep :type Boolean) (SweepResult :type Hit%20Result%20Structure%20%28by%20ref%29))
  (bind _asbp_structure_destructible (Utilities|Casting|CastToBP_Structure_Destructible OtherActor))
  (Default|ApplyDamageTornadoInitiation _asbp_structure_destructible (Variables|Default|GetDamageValue)))

(event OnComponentEndOverlap(Capsule)
  (params (OverlappedComponent :type Primitive%20Component%20Object%20Reference) (OtherActor :type Actor%20Object%20Reference) (OtherComp :type Primitive%20Component%20Object%20Reference) (OtherBodyIndex :type Integer))
  (bind _asbp_structure_destructible (Utilities|Casting|CastToBP_Structure_Destructible OtherActor))
  (Default|ApplyDamageTornadoStop _asbp_structure_destructible))

(event Custom|MovementTick
  (bind _currentdirection (Variables|Default|GetCurrentDirection))
  (bind _speed (Variables|Default|GetSpeed))
  (bind _root (Variables|Default|GetRoot))
  (bind _returnvalue (Transformation|GetWorldLocation _root))
  (bind _returnvalue_2 (* _currentdirection _speed))
  (bind _returnvalue_3 (+ _returnvalue _returnvalue_2))
  (bind (_outhit _returnvalue_4) (Collision|LineTraceByChannel (+ _returnvalue_3 "0,0,500.000000") (- _returnvalue_3 "0,0,1000.000000") "TraceTypeQuery1" true 0 "None" true "(R=1.000000,G=0.000000,B=0.007289,A=1.000000)"))
  (if _returnvalue_4
    (Transformation|AddActorWorldOffset (- (.Location (Collision|BreakHitResult _outhit)) (Transformation|GetWorldLocation (Variables|Default|GetRoot))) false true)
    (else
      (Variables|Default|SetInitialDirection (Math|Vector|Normalize (Math|Vector|ProjectVectorontoPlane (Math|Random|RandomUnitVector) "0, 0,1.000000"))))))

(event Custom|DeathTimer
  (Utilities|FlowControl|Delay (Variables|Default|GetLifeDuration))
  (Actor|DestroyActor))

(event EventBeginPlay
  (Utilities|FlowControl|DelayUntilNextTick)
  (CallFunction|DeathTimer)
  (Utilities|Time|SetTimerbyEvent (delegate Custom|MovementTick) 0.05 true)
  (Variables|Default|SetCurrentDirection (Variables|Default|GetInitialDirection)))

(event EventTick
  (params (DeltaSeconds :type Float%20%28single-precision%29))
  ;[1 1 1] Direction Noise
  (if (== (Math|Random|RandomIntegerinRange 1 20) 1)
    (Variables|Default|SetCurrentDirection (Math|Vector|RotateVectorAroundAxis (Variables|Default|GetInitialDirection) (* (Class|KismetAnimationLibrary|MakePerlinNoiseandRemap (Math|Random|RandomFloatinRange -1.0 1.0) -45.0 45.0) 1.5) "0, 0,1.000000"))))

(fn ConstructionScript)