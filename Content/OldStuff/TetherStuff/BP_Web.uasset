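; BP_Web is a cable tether joining two hit points, pulling attached physics objects with spring forces.
; A looping 0.01s timer applies stretch-based forces, tints the cable by tension and reports overstretch to the player.
; It breaks into Niagara effects after sustained overstretch or when either hit actor becomes invalid.
; Its Powered state latches on for BP_MagicConduit connections, otherwise copies an attached BP_PhysicsObject each Tick.
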(event Custom|TetherBreak
  ;[1 1 1] Tether Break
  (Development|PrintString "Tether Break")
  (for _array_element (Class|CableComponent|GetCableParticleLocations (Variables|Default|GetCable))
    (Niagara|SpawnSystematLocation "/Game/VFX/NS_WebBreak_System.NS_WebBreak_System" _array_element))
  (Actor|DestroyActor))

(event Custom|PhysicsTick_Event
  (bind _playerref (Variables|Default|GetPlayerRef))
  (bind _rootdynamicobject (Variables|Default|GetRootDynamicObject))
  (bind _connecteddynamicobject (Variables|Default|GetConnectedDynamicObject))
  (bind _secondhitresult (Variables|Default|GetSecondHitResult))
  (bind _rootdynamicobject_2 (Variables|Default|GetRootDynamicObject))
  (bind _connecteddynamicobject_2 (Variables|Default|GetConnectedDynamicObject))
  (bind _rootdynamicobject_3 (Variables|Default|GetRootDynamicObject))
  (bind _connecteddynamicobject_3 (Variables|Default|GetConnectedDynamicObject))
  (bind _firsthitresult (Variables|Default|GetFirstHitResult))
  (bind _location (Collision|BreakHitResult _firsthitresult))
  (bind _location_2 (Collision|BreakHitResult _secondhitresult))
  (bind _rootcomponent (Variables|/Script/Engine.Actor|GetRootComponent _connecteddynamicobject_2))
  (bind _rootcomponent_2 (Variables|/Script/Engine.Actor|GetRootComponent _rootdynamicobject))
  (bind _rootcomponent_3 (Variables|/Script/Engine.Actor|GetRootComponent _connecteddynamicobject))
  (bind _rootcomponent_4 (Variables|/Script/Engine.Actor|GetRootComponent _rootdynamicobject_2))
  (bind _rootcomponent_5 (Variables|/Script/Engine.Actor|GetRootComponent _connecteddynamicobject_3))
  (bind _rootcomponent_6 (Variables|/Script/Engine.Actor|GetRootComponent _rootdynamicobject_3))
  (bind _returnvalue (Transformation|GetWorldLocation _rootcomponent))
  (bind _returnvalue_2 (Transformation|GetWorldLocation _rootcomponent_5))
  (bind _returnvalue_3 (Transformation|GetWorldLocation _rootcomponent_2))
  (bind _returnvalue_4 (Transformation|GetWorldLocation _rootcomponent_4))
  (bind _returnvalue_5 (Transformation|GetWorldLocation _rootcomponent_3))
  (bind _returnvalue_6 (Transformation|GetWorldLocation _rootcomponent_6))
  (bind _returnvalue_7 (- _returnvalue_2 _returnvalue_4))
  (bind _returnvalue_8 (- _returnvalue _location))
  (bind _returnvalue_9 (- _returnvalue_3 _location_2))
  (bind _returnvalue_10 (- _returnvalue_6 _returnvalue_5))
  (Utilities|FlowControl|Sequence
    (:then_0
      (if (Variables|Default|GetPullable)
        (if (Variables|Default|GetRootPullable)
          (Variables|Default|SetConnectionDirection (* _returnvalue_7 -1))
          (Variables|Default|SetCurrentDistance (Math|Vector|VectorLength _returnvalue_7))
          (else
            (Variables|Default|SetConnectionDirection (* _returnvalue_8 -1))
            (Variables|Default|SetCurrentDistance (Math|Vector|VectorLength _returnvalue_8))))
        (if (> (Variables|Default|GetCurrentDistance) (- (Variables|Default|GetInitialDistance) 1e+02))
          (bind _asprimitive_component (Utilities|Casting|CastToPrimitiveComponent (Variables|/Script/Engine.Actor|GetRootComponent (Variables|Default|GetConnectedDynamicObject)))
            (:then
              (if (> (Variables|Default|GetCurrentDistance) (Variables|Default|GetMaxConnectionDistance))
                (Physics|AddForce _asprimitive_component (* (* (Variables|Default|GetConnectionDirection) (Variables|Default|GetSpringConstant)) (* (- (Variables|Default|GetMaxConnectionDistance) (Variables|Default|GetInitialDistance)) (Variables|Default|GetForceScalar))) "None" false)
                (else
                  (Physics|AddForce _asprimitive_component (* (* (Variables|Default|GetConnectionDirection) (Variables|Default|GetSpringConstant)) (* (- (Variables|Default|GetCurrentDistance) (Variables|Default|GetInitialDistance)) (Variables|Default|GetForceScalar))) "None" false))))
            (:CastFailed
              (Development|PrintString "CAST FAILED IN WEB"))))))
    (:then_1
      (if (Variables|Default|GetRootPullable)
        (if (Variables|Default|GetPullable)
          (Variables|Default|SetConnectionDirection (* _returnvalue_10 -1))
          (Variables|Default|SetCurrentDistance (Math|Vector|VectorLength _returnvalue_10))
          (else
            (Variables|Default|SetConnectionDirection (* _returnvalue_9 -1))
            (Variables|Default|SetCurrentDistance (Math|Vector|VectorLength _returnvalue_9))))
        (if (> (Variables|Default|GetCurrentDistance) (Variables|Default|GetInitialDistance))
          (bind _asprimitive_component_2 (Utilities|Casting|CastToPrimitiveComponent (Variables|/Script/Engine.Actor|GetRootComponent (Variables|Default|GetRootDynamicObject)))
            (:then
              (if (> (Variables|Default|GetCurrentDistance) (Variables|Default|GetMaxConnectionDistance))
                (Physics|AddForce _asprimitive_component_2 (* (* (Variables|Default|GetConnectionDirection) (Variables|Default|GetSpringConstant)) (* (* (- (Variables|Default|GetMaxConnectionDistance) (Variables|Default|GetInitialDistance)) (Variables|Default|GetForceScalar)) -1.0)) "None" false)
                (else
                  (Physics|AddForce _asprimitive_component_2 (* (* (Variables|Default|GetConnectionDirection) (Variables|Default|GetSpringConstant)) (* (- (Variables|Default|GetCurrentDistance) (Variables|Default|GetInitialDistance)) (Variables|Default|GetForceScalar))) "None" false))))
            (:CastFailed
              (Development|PrintString "CAST FAILED IN WEB"))))))
    (:then_2
      (Rendering|Material|SetVectorParameterValue (Variables|Default|GetDynamicMaterial) "Fresnel_Color" (Math|Color|Lerp(LinearColor) (Variables|Default|GetColorBase) (Variables|Default|GetColorTension) (/ (- (Variables|Default|GetCurrentDistance) (Variables|Default|GetInitialDistance)) (- (Variables|Default|GetMaxConnectionDistance) (Variables|Default|GetInitialDistance)))) :!class /Script/Engine.MaterialInstanceDynamic)
      (Utilities|IsValid _playerref
        (:Is%20Valid
          (if (> (Variables|Default|GetCurrentDistance) (Variables|Default|GetMaxConnectionDistance))
            (Default|MaxTension _playerref true (Math|Float|MapRangeClamped (- (Variables|Default|GetCurrentDistance) (Variables|Default|GetMaxConnectionDistance)) 0.0 1e+02 0.0 1.0))
            (Utilities|FlowControl|DoOnce false :!label _label
              (:Completed
                (Utilities|FlowControl|RetriggerableDelay 2.0)
                (if (> (Variables|Default|GetCurrentDistance) (Variables|Default|GetMaxConnectionDistance))
                  (Default|MaxTension _playerref false 0.0)
                  (CallFunction|TetherBreak))))
            (else
              (Default|MaxTension _playerref false 0.0)
              (goto _label Reset))))
        (:Is%20Not%20Valid
          (Development|PrintString "NOT VALID PLAYER REF" true true "(R=1.000000,G=0.012011,B=0.000000,A=1.000000)"))))
    (:then_3
      (Utilities|FlowControl|Sequence
        (:then_0
          (Utilities|IsValid (.HitActor (Collision|BreakHitResult (Variables|Default|GetSecondHitResult)))
            (:Is%20Not%20Valid
              _)))
        (:then_1
          (Utilities|IsValid (.HitActor (Collision|BreakHitResult (Variables|Default|GetFirstHitResult)))
            (:Is%20Not%20Valid
              _))))
      (CallFunction|TetherBreak))))

(event Custom|PhysicsTickTimer
  (CallFunction|PhysicsTickEvent))

(event EventBeginPlay
  (bind _rootdynamicobject (Variables|Default|GetRootDynamicObject))
  (bind _secondhitresult (Variables|Default|GetSecondHitResult))
  (bind (_bblockinghit _binitialoverlap _time _distance _location _impactpoint _normal _impactnormal _physmat _hitactor _hitcomponent) (Collision|BreakHitResult _secondhitresult))
  (Utilities|FlowControl|DelayUntilNextTick)
  (Utilities|Time|SetTimerbyEvent (delegate Custom|PhysicsTickTimer) 0.01 true)
  (Utilities|FlowControl|Sequence
    (:then_1
      (if (Physics|IsSimulatingPhysics _hitcomponent "None")
        (bind _output_get (Variables|Default|SetConnectedDynamicObject _hitactor))
        (Class|CableComponent|SetAttachEndto (Variables|Default|GetCable) _output_get "None" "None")
        (Variables|Default|SetPullable true)
        (Development|PrintString (Utilities|GetDisplayName _output_get) true true "(R=0.000000,G=1.000000,B=0.314280,A=1.000000)")
        (else
          (Variables|/Script/CableComponent.CableComponent|SetEndLocation (Variables|Default|GetCable) (- (.Location (Collision|BreakHitResult (Variables|Default|GetSecondHitResult))) (.Location (Collision|BreakHitResult (Variables|Default|GetFirstHitResult))))))))
    (:then_2
      (bind _output_get_2 (Variables|Default|SetInitialDistance (Math|Vector|VectorLength (- (.Location (Collision|BreakHitResult (Variables|Default|GetSecondHitResult))) (.Location (Collision|BreakHitResult (Variables|Default|GetFirstHitResult)))))))
      (Variables|Default|SetMaxConnectionDistance (* _output_get_2 5.0))
      (bind _output_get_3 (Variables|/Script/CableComponent.CableComponent|SetCableLength (Variables|Default|GetCable) (Math|Float|Lerp 2e+01 (Variables|Default|GetMaxCableLength) (Math|Float|Clamp(Float) (/ _output_get_2 (Variables|Default|GetMaxTensionDistance)))))))
    (:then_3
      (Utilities|IsValid (Variables|Default|GetRootDynamicObject)
        (:Is%20Valid
          (if (Physics|IsSimulatingPhysics (Variables|/Script/Engine.Actor|GetRootComponent _rootdynamicobject) "None")
            (Variables|Default|SetRootPullable true)
            (else
              (Development|PrintString (Utilities|GetDisplayName _rootdynamicobject) true true "(R=0.070989,G=0.000000,B=1.000000,A=1.000000)"))))))
    (:then_4
      (Utilities|Casting|CastToBP_MagicConduit (.HitActor (Collision|BreakHitResult (Variables|Default|GetFirstHitResult)))
        (:then
          (Variables|Default|SetPowered true))
        (:CastFailed
          (Utilities|Casting|CastToBP_MagicConduit (.HitActor (Collision|BreakHitResult (Variables|Default|GetSecondHitResult))))
          (Variables|Default|SetPowered true)))
      (Variables|Default|SetMagicConduitConnected true))))

(event EventTick
  (params (DeltaSeconds :type Float%20%28single-precision%29))
  (if (Variables|Default|GetMagicConduitConnected)
    (Development|PrintString (Utilities|String|ToString(Boolean) (Variables|Default|GetPowered)) true true "(R=1.000000,G=0.258376,B=0.000000,A=1.000000)" 0.01 :!label _label)
    (else
      (bind _asbp_physics_object (Utilities|Casting|CastToBP_PhysicsObject (.HitActor (Collision|BreakHitResult (Variables|Default|GetFirstHitResult))))
        (:then
          (Variables|Default|SetPowered (Variables|/Game/EnvironmentActors/OldGame/BP_PhysicsObject.BP_PhysicsObject_C|GetPowered _asbp_physics_object))
          (goto _label))
        (:CastFailed
          (bind _asbp_physics_object_2 (Utilities|Casting|CastToBP_PhysicsObject (.HitActor (Collision|BreakHitResult (Variables|Default|GetSecondHitResult))))
            (:then
              (Variables|Default|SetPowered (Variables|/Game/EnvironmentActors/OldGame/BP_PhysicsObject.BP_PhysicsObject_C|GetPowered _asbp_physics_object_2))
              (goto _label))
            (:CastFailed
              (Variables|Default|SetPowered false)
              (Variables|Default|SetMagicConduitConnected false))))))))

(fn ConstructionScript
  (bind _returnvalue (Rendering|Material|CreateDynamicMaterialInstance (Variables|Default|GetCable) 0 0 "None" :!class /Script/Engine.PrimitiveComponent))
  (Variables|Default|SetDynamicMaterial _returnvalue))