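; BP_Gate is a gate actor that opens by sinking vertically and closes by rising back.
; BeginPlay caches the root component's world location as the closed position.
; OpenGate_Event plays a timeline that eases the root's Z down by a fixed offset, and CloseGate_Event reverses that timeline.
; Each update sets world location and rotation together, with only the location specified.
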(event Custom|OpenGate_Event
  (bind _worldlocation (Variables|Default|GetWorldLocation))
  (bind _alpha (Timeline|Timeline_0 Play)
    (:Update
      (Transformation|SetWorldLocationAndRotation (Variables|Default|GetDefaultSceneRoot) (Math|Vector|MakeVector (.x _worldlocation) (.y _worldlocation) (Class|KismetMathLibrary|FInterpEaseinOut (.z _worldlocation) (- (.z _worldlocation) 2.5e+02) _alpha 1.0)) "0, 0, 0" false false))))

(event Custom|CloseGate_Event
  (bind _worldlocation (Variables|Default|GetWorldLocation))
  (bind _alpha (Timeline|Timeline_0 Reverse)
    (:Update
      (Transformation|SetWorldLocationAndRotation (Variables|Default|GetDefaultSceneRoot) (Math|Vector|MakeVector (.x _worldlocation) (.y _worldlocation) (Class|KismetMathLibrary|FInterpEaseinOut (.z _worldlocation) (- (.z _worldlocation) 2.5e+02) _alpha 1.0)) "0, 0, 0" false false))))

(event EventBeginPlay
  (Utilities|FlowControl|Sequence
    (:then_0
      (Variables|Default|SetWorldLocation (Transformation|GetWorldLocation (Variables|Default|GetDefaultSceneRoot))))))

(fn ConstructionScript)