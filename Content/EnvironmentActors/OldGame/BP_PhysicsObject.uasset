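; Physics object for the environment, with a configurable mesh and a Powered state taken from attached webs.
; The construction script applies the mesh and feeds MassKg into the static mesh's mass scale rather than a kilogram override.
; Each tick pins the collider to zero world rotation, then copies Powered from directly attached BP_Web actors.
; The last web visited wins, and the reset to false is unconnected, so Powered persists without webs.
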(event EventTick
  (params (DeltaSeconds :type Float%20%28single-precision%29))
  (Utilities|FlowControl|Sequence
    (:then_0
      (Transformation|SetWorldRotation (Variables|Default|GetCollider) "0, 0, 0" false false))
    (:then_1
      (for _array_element (Actor|GetAttachedActors true false)
        (bind _asbp_web (Utilities|Casting|CastToBP_Web _array_element))
        (Variables|Default|SetPowered (Variables|/Game/OldStuff/TetherStuff/BP_Web.BP_Web_C|GetPowered _asbp_web))))))

(fn ConstructionScript
  (bind _staticmesh (Variables|Default|GetStaticMesh))
  (Components|StaticMesh|SetStaticMesh _staticmesh (Variables|Default|GetMesh))
  (Class|PrimitiveComponent|SetAllMassScale _staticmesh (Variables|Default|GetMass%20%28kg%29)))