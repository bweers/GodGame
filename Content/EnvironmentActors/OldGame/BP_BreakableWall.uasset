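; BP_BreakableWall is a wall actor that breaks when a fast-moving BP_PhysicsObject overlaps it.
; On overlap it compares the object's speed to a hard-coded threshold, then spawns the NS_WallBreak_System Niagara effect at its Cube's location and destroys itself.
; Debug prints show the speed and the name of the object's first attached actor on every such overlap, whether or not the wall breaks.
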(event Collision|EventActorBeginOverlap
  (params (OtherActor :type Actor%20Object%20Reference))
  (bind _asbp_physics_object (Utilities|Casting|CastToBP_PhysicsObject OtherActor))
  (Development|PrintString (Utilities|String|ToString(Float) (Math|Vector|VectorLength (Transformation|GetVelocity _asbp_physics_object))) true true "(R=0.024143,G=1.000000,B=0.000000,A=1.000000)" 1e+01)
  (Development|PrintString (Utilities|GetDisplayName (Utilities|Array|Get(acopy) (Actor|GetAttachedActors _asbp_physics_object true false))))
  (if (> (Math|Vector|VectorLength (Transformation|GetVelocity _asbp_physics_object)) 1.8e+03)
    (Niagara|SpawnSystematLocation "/Game/VFX/NS_WallBreak_System.NS_WallBreak_System" (Transformation|GetWorldLocation (Variables|Default|GetCube)))
    (Actor|DestroyActor)))

(fn ConstructionScript)