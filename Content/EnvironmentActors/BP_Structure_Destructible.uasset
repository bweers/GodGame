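; Destructible structure actor that loses health from impacts, direct damage calls and tornado exposure.
; Impact velocity selects light or heavy damage, while tornado damage repeats on a looping timer using IncomingTornadoDamage, ignoring the passed DamageValue.
; Each hit updates a FullHealth, Damaged or Destroyed state from health.
; Tick applies that state by squashing the actor's scale and, when destroyed, disabling collision and spawning a one-time Niagara wall-break effect.
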(event Custom|ApplyDamage_Velocity
  (params (Velocity :type Float%20%28double-precision%29))
  (if (> Velocity 6.5e+02)
    (Variables|Default|SetStructureHealth (- (Variables|Default|GetStructureHealth) 100))
    (CallFunction|UpdateState :!label _label)
    (elif (> Velocity 5e+01)
      (Variables|Default|SetStructureHealth (- (Variables|Default|GetStructureHealth) 55))
      (goto _label))))

(event Custom|ApplyDamage_Value
  (params (Value :type Integer))
  (Variables|Default|SetStructureHealth (- (Variables|Default|GetStructureHealth) Value))
  (CallFunction|UpdateState))

(event Custom|UpdateState
  (if (>= (Variables|Default|GetStructureHealth) 100)
    (Variables|Default|SetState "NewEnumerator0")
    (elif (<= (Variables|Default|GetStructureHealth) 0)
      (Variables|Default|SetState "NewEnumerator2")
      (else
        (Variables|Default|SetState "NewEnumerator1")))))

(event Custom|ApplyDamage_Tornado_Initiation
  (params (DamageValue :type Integer))
  (bind _returnvalue (Utilities|Time|SetTimerbyEvent (delegate Custom|ApplyDamage_Tornado_Tick) 0.2 true)))

(event Custom|ApplyDamage_Tornado_Tick
  (bind _incomingtornadodamage (Variables|Default|GetIncomingTornadoDamage))
  (Variables|Default|SetStructureHealth (- (Variables|Default|GetStructureHealth) _incomingtornadodamage))
  (CallFunction|UpdateState)
  (Development|PrintString (Utilities|String|ToString(Integer) _incomingtornadodamage) true true "(R=1.000000,G=0.000000,B=0.045170,A=1.000000)" 0.5))

(event Custom|ApplyDamage_Tornado_Stop
  (Utilities|Time|ClearandInvalidateTimerbyHandle (stale Custom|ApplyDamage_Tornado_Initiation _returnvalue)))

(event EventTick
  (params (DeltaSeconds :type Float%20%28single-precision%29))
  (switch Utilities|FlowControl|Switch|SwitchonENum_StructureState (Variables|Default|GetState)
    (:NewEnumerator1
      (Transformation|SetActorScale3D "0.700000,0.700000,0.800000"))
    (:NewEnumerator2
      (Transformation|SetActorScale3D "0.700000,0.700000,0.100000")
      (Collision|SetCollisionEnabled (Variables|Default|GetStructure) "NoCollision")
      (Utilities|FlowControl|DoOnce false
        (:Completed
          (bind _returnvalue (Niagara|SpawnSystematLocation "/Game/VFX/NS_WallBreak_System.NS_WallBreak_System" (Transformation|GetWorldLocation (Variables|Default|GetScene)) "0, 0, 0" "1.000000,1.000000,1.000000" false)))))))

(fn ConstructionScript)